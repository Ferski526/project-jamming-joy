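; BP_CrystalButton is a crystal button actor that the player presses by shooting it with a FirstPersonProjectile.
; On BeginPlay it creates a dynamic material instance for its static mesh.
; A projectile hit sets IsPressed, calls the OnPressed dispatcher for listeners and raises the material's Emissive parameter to make it glow.
; Nothing resets the pressed state, and a constant-true branch leaves the missing-tag debug print unreachable.
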(event EventBeginPlay
  (bind _returnvalue (Rendering|Material|CreateDynamicMaterialInstance (Variables|Default|GetStaticMesh) 0 0 "None" :!class /Script/Engine.PrimitiveComponent))
  (bind _output_get (Variables|Default|SetDynMat _returnvalue))
  (Rendering|Material|SetMaterial (Variables|Default|GetStaticMesh) 0 _output_get))

(event Collision|EventActorBeginOverlap
  (params (OtherActor :type Actor%20Object%20Reference)))

(event EventTick
  (params (DeltaSeconds :type Float%20%28single-precision%29)))

(event Collision|EventHit
  (params (MyComp :type Primitive%20Component%20Object%20Reference) (Other :type Actor%20Object%20Reference) (OtherComp :type Primitive%20Component%20Object%20Reference) (bSelfMoved :type Boolean) (HitLocation :type Vector :default "0, 0, 0") (HitNormal :type Vector :default "0, 0, 0") (NormalImpulse :type Vector :default "0, 0, 0") (Hit :type Hit%20Result%20Structure%20%28by%20ref%29))
  (Utilities|Casting|CastToFirstPersonProjectile Other)
  (if (Utilities|IsValid Other)
    (Utilities|Casting|CastToFirstPersonProjectile Other)
    (if true
      (Variables|Default|SetbIsPressed true)
      (Default|CallOnPressedDispatcher)
      (Rendering|Material|SetScalarParameterValue (Variables|Default|GetDynMat) "Emissive" 1e+02 :!class /Script/Engine.MaterialInstanceDynamic)
      (else
        (Development|PrintString "I don't have tag")))))

(fn ConstructionScript)