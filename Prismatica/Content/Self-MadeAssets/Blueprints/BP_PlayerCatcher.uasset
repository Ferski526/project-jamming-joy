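; BP_PlayerCatcher is a trigger volume that sends the player back to a respawn point on entering it.
; When the Box component begins an overlap with a FirstPersonCharacter, it moves that character to the RespawnPoint component's world location and ignores other actors.
; The construction script applies the RespawnPointOffset and BoxSize variables to the respawn point's relative location and the box extent.
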(event OnComponentBeginOverlap(Box)
  (params (OverlappedComponent :type Primitive%20Component%20Object%20Reference) (OtherActor :type Actor%20Object%20Reference) (OtherComp :type Primitive%20Component%20Object%20Reference) (OtherBodyIndex :type Integer) (bFromSweep :type Boolean) (SweepResult :type Hit%20Result%20Structure%20%28by%20ref%29))
  (bind _asfirst_person_character (Utilities|Casting|CastToFirstPersonCharacter OtherActor))
  (Transformation|SetActorLocation _asfirst_person_character (Transformation|GetWorldLocation (Variables|Default|GetRespawnPoint)) false false))

(event EventBeginPlay)

(event Collision|EventActorBeginOverlap
  (params (OtherActor :type Actor%20Object%20Reference)))

(event EventTick
  (params (DeltaSeconds :type Float%20%28single-precision%29)))

(fn ConstructionScript
  (Utilities|FlowControl|Sequence
    (:then_0
      (Transformation|SetRelativeLocation (Variables|Default|GetRespawnPoint) (Variables|Default|GetRespawnPointOffset) false false))
    (:then_1
      (Components|Box|SetBoxExtent (Variables|Default|GetBox) (Variables|Default|GetBoxSize) true))))