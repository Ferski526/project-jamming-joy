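; Final level trigger actor that ends the game with a fade, end credits and a switch to TargetLevelName.
; On any overlap, checking only the player character rather than the overlapping actor, it writes TargetLevelName into a fresh BP_SaveGameProgress and saves it to the progress slot.
; It then plays WBP_FadeToBlack, whose finished event shows WBP_EndCredits and opens the target level after a fixed delay.
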(event Custom|ShowEndMessage
  (bind _returnvalue (UserInterface|CreateWidget "/Game/Self-MadeAssets/UI/Widgets/WBP_EndCredits.WBP_EndCredits_C"))
  (UserInterface|Viewport|AddtoViewport _returnvalue 0)
  (Utilities|FlowControl|Delay 7.0)
  (Game|OpenLevel(byName) (Variables|Default|GetTargetLevelName)))

(event EventBeginPlay)

(event Collision|EventActorBeginOverlap
  (params (OtherActor :type Actor%20Object%20Reference))
  (Utilities|Casting|CastToCharacter (Game|GetPlayerCharacter 0))
  (bind _returnvalue (SaveGame|CreateSaveGameObject "/Game/Self-MadeAssets/GameInstance/BP_SaveGameProgress.BP_SaveGameProgress_C"))
  (bind _asbp_save_game_progress (Utilities|Casting|CastToBP_SaveGameProgress _returnvalue))
  (Variables|/Game/Self-MadeAssets/GameInstance/BP_SaveGameProgress.BP_SaveGameProgress_C|SetLastLevelName _asbp_save_game_progress (Variables|Default|GetTargetLevelName))
  (SaveGame|SaveGametoSlot _asbp_save_game_progress "SaveSlot_Progress")
  (bind _returnvalue_2 (UserInterface|CreateWidget "/Game/Self-MadeAssets/UI/Widgets/WBP_FadeToBlack.WBP_FadeToBlack_C"))
  (bind _aswbp_fade_to_black (Utilities|Casting|CastToWBP_FadeToBlack _returnvalue_2))
  (UserInterface|Viewport|AddtoViewport _returnvalue_2 0)
  (Default|PlayFadetoBlack _aswbp_fade_to_black)
  (EventDispatchers|BindEventtoOnFadetoBlackFinished _aswbp_fade_to_black (delegate Custom|ShowEndMessage)))

(event EventTick
  (params (DeltaSeconds :type Float%20%28single-precision%29)))

(fn ConstructionScript)