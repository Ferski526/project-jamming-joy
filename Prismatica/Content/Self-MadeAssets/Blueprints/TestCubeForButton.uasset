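; A test cube actor that changes color when a referenced activator, such as a button, is pressed.
; On BeginPlay it creates a dynamic instance of M_CubeColor for the cube mesh and, if ActivatorReference is valid, binds to its OnPressedDispatcher.
; OnButtonPressed sets the instance's Color parameter to cyan, with no logic to revert it.
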(event Custom|OnButtonPressed
  (Rendering|Material|SetVectorParameterValue (Variables|Default|GetDynamicMatInstance) "Color" "(R=0.000000,G=1.000000,B=0.851157,A=1.000000)" :!class /Script/Engine.MaterialInstanceDynamic))

(event EventBeginPlay
  (Utilities|FlowControl|Sequence
    (:then_0
      (bind _returnvalue (Rendering|Material|CreateDynamicMaterialInstance (Variables|Default|GetCube) 0 "/Game/Self-MadeAssets/Blueprints/M_CubeColor.M_CubeColor" "None" :!class /Script/Engine.PrimitiveComponent))
      (bind _output_get (Variables|Default|SetDynamicMatInstance _returnvalue))
      (Rendering|Material|SetMaterial (Variables|Default|GetCube) 0 _output_get))
    (:then_1
      (if (Utilities|IsValid (Variables|Default|GetActivatorReference))
        (EventDispatchers|BindEventtoOnPressedDispatcher (Variables|Default|GetActivatorReference) (EventDispatchers|CreateEvent :!event Custom|OnButtonPressed))))))

(event Collision|EventActorBeginOverlap
  (params (OtherActor :type Actor%20Object%20Reference)))

(event EventTick
  (params (DeltaSeconds :type Float%20%28single-precision%29)))

(fn ConstructionScript)