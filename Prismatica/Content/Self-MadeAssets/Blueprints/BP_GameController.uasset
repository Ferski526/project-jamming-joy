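; BP_GameController is a controller Blueprint that handles pausing and loading-screen display for the local player.
; The PauseGame input, only while the game is unpaused, pauses it, creates and stores WBP_PauseMenu, then switches to UI-only input with a visible cursor.
; The ShowLoadingScreen event adds WBP_LoadingScreen to the viewport with UI-only input and a hidden cursor.
; It contains no unpause or widget-removal logic.
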(event Custom|ShowLoadingScreen
  (bind _returnvalue (UserInterface|CreateWidget "/Game/Self-MadeAssets/UI/Widgets/WBP_LoadingScreen.WBP_LoadingScreen_C"))
  (UserInterface|Viewport|AddtoViewport _returnvalue 0)
  (Input|SetInputModeUIOnly (Game|GetPlayerController 0) 0 "DoNotLock")
  (Variables|Default|SetbShowMouseCursor false))

(event EventBeginPlay)

(event EventTick
  (params (DeltaSeconds :type Float%20%28single-precision%29)))

(event Input|ActionEvents|InputActionPauseGame
  (params (Key :type Key%20Structure))
  ;[1 1 1] GamePausing
  (:Pressed
    (if (not (Game|IsGamePaused))
      (Game|SetGamePaused true)
      (bind _returnvalue (UserInterface|CreateWidget "/Game/Self-MadeAssets/UI/Widgets/WBP_PauseMenu.WBP_PauseMenu_C"))
      (bind _output_get (Variables|Default|SetPauseMenuWidget _returnvalue))
      (UserInterface|Viewport|AddtoViewport _output_get 0)
      (Input|SetInputModeUIOnly (Game|GetPlayerController 0) 0 "DoNotLock")
      (Variables|Default|SetbShowMouseCursor true))))

(fn ConstructionScript)