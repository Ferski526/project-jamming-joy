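; Moving platform that, once activated, shuttles back and forth between a start and an end location.
; A press dispatcher on the linked BP_UniversalButton sets it active, and nothing here switches it off again.
; Tick eases it toward the current target with VInterpTo and flips direction when within a small distance.
; The construction script places two arrow components at the endpoints.
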(event Custom|ActivatePlatform
  (Variables|Default|SetisActive true))

(event EventBeginPlay
  (bind _activateactor (Variables|Default|GetActivateActor))
  (if (Utilities|IsValid _activateactor)
    (bind _asbp_universal_button (Utilities|Casting|CastToBP_UniversalButton _activateactor))
    (EventDispatchers|BindEventtoOnPressedDispatcher _asbp_universal_button (delegate Custom|ActivatePlatform))))

(event Collision|EventActorBeginOverlap
  (params (OtherActor :type Actor%20Object%20Reference)))

(event EventTick
  (params (DeltaSeconds :type Float%20%28single-precision%29))
  (if (Variables|Default|GetisActive)
    (Transformation|SetActorLocation (Math|Interpolation|VInterpTo (Transformation|GetActorLocation) (select (Variables|Default|GetMoveDirection) (Variables|Default|GetEndLocation) (Variables|Default|GetStartLocation)) DeltaSeconds (Variables|Default|GetInterpSpeed)) false false)
    (if (<= (Math|Vector|Distance(Vector) (select (Variables|Default|GetMoveDirection) (Variables|Default|GetEndLocation) (Variables|Default|GetStartLocation)) (Math|Interpolation|VInterpTo (Transformation|GetActorLocation) (select (Variables|Default|GetMoveDirection) (Variables|Default|GetEndLocation) (Variables|Default|GetStartLocation)) DeltaSeconds (Variables|Default|GetInterpSpeed))) 5.0)
      (Variables|Default|SetMoveDirection (not (Variables|Default|GetMoveDirection))))))

(fn ConstructionScript
  (Utilities|FlowControl|Sequence
    (:then_0
      (Transformation|SetWorldLocation (Variables|Default|GetStartArrow) (Variables|Default|GetStartLocation) false false))
    (:then_1
      (Transformation|SetWorldLocation (Variables|Default|GetEndArrow) (Variables|Default|GetEndLocation) false false))))