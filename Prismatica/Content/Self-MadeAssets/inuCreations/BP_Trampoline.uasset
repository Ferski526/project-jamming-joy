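; Trampoline actor that launches an overlapping FirstPersonCharacter upward, but only while active.
; On BeginPlay it creates a dynamic material on one Platform slot and binds to the pressed dispatcher of its ActivateActor, if that is a BP_UniversalButton.
; OnPressed sets it active and raises the material's emissive, with nothing here switching it back off.
; The launch adds to existing velocity rather than overriding it, and debug prints remain.
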(event Custom|OnPressed
  (Variables|Default|SetisActive true)
  (Rendering|Material|SetScalarParameterValue (Variables|Default|GetDynMat) "Emissive" 1e+02 :!class /Script/Engine.MaterialInstanceDynamic))

(event EventBeginPlay
  (bind _activateactor (Variables|Components|GetActivateActor))
  (Utilities|FlowControl|Sequence
    (:then_0
      (bind _returnvalue (Rendering|Material|CreateDynamicMaterialInstance (Variables|Default|GetPlatform) 2 0 "None" :!class /Script/Engine.PrimitiveComponent))
      (bind _output_get (Variables|Default|SetDynMat _returnvalue))
      (Rendering|Material|SetMaterial (Variables|Default|GetPlatform) 2 _output_get))
    (:then_1
      (if (Utilities|IsValid _activateactor)
        (bind _asbp_universal_button (Utilities|Casting|CastToBP_UniversalButton _activateactor))
        (EventDispatchers|BindEventtoOnPressedDispatcher _asbp_universal_button (EventDispatchers|CreateEvent :!event Custom|OnPressed))))))

(event Collision|EventActorBeginOverlap
  (params (OtherActor :type Actor%20Object%20Reference))
  (Development|PrintString "trampolina overlap")
  (if (Variables|Default|GetisActive)
    (Development|PrintString "trampolina aktywna firing")
    (bind _asfirst_person_character (Utilities|Casting|CastToFirstPersonCharacter OtherActor))
    (Character|LaunchCharacter _asfirst_person_character "0, 0,1500.000000" false false)))

(fn ConstructionScript)