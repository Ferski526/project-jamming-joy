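; A holographic door that toggles between solid and passable when its linked universal or crystal button is pressed.
; On BeginPlay it creates a dynamic material and binds to the press dispatcher of the assigned ActivateActor.
; Each toggle uses a FlipFlop to switch collision and play or reverse a timeline driving the material's "Fade Out" parameter.
; When StartVisible is false, it fires one toggle at startup to begin open.
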(event Custom|OnButtonPressed
  (Utilities|FlowControl|FlipFlop
    (:A
      (Collision|SetCollisionEnabled (Variables|Default|GetHoloDoor) "NoCollision")
      (bind _newtrack_0 (Timeline|Fade%20Time PlayFromStart)
        (:Update
          (Rendering|Material|SetScalarParameterValue (stale EventBeginPlay _returnvalue) "Fade Out" (Math|Float|Lerp 1.0 0.0 _newtrack_0) :!class /Script/Engine.MaterialInstanceDynamic))))
    (:B
      (Collision|SetCollisionEnabled (Variables|Default|GetHoloDoor) "QueryAndPhysics")
      (Timeline|Fade%20Time ReverseFromEnd))))

(event EventBeginPlay
  (bind _activateactor (Variables|Components|GetActivateActor))
  (if (Variables|Default|GetbStartVisible?)
    _
    (else
      (CallFunction|OnButtonPressed)))
  (Utilities|FlowControl|Sequence
    (:then_0
      (Input|EnableInput (Game|GetPlayerController 0))
      (bind _returnvalue (Rendering|Material|CreateDynamicMaterialInstance (Variables|Default|GetHoloDoor) 0 "/Game/Self-MadeAssets/inuCreations/M_HoloDrzwi.M_HoloDrzwi" "None" :!class /Script/Engine.PrimitiveComponent)))
    (:then_1
      (if (Utilities|IsValid (Variables|Components|GetActivateActor))
        (bind _asbp_universal_button (Utilities|Casting|CastToBP_UniversalButton _activateactor)
          (:then
            (EventDispatchers|BindEventtoOnPressedDispatcher _asbp_universal_button (EventDispatchers|CreateEvent :!event Custom|OnButtonPressed)))
          (:CastFailed
            (bind _asbp_crystal_button (Utilities|Casting|CastToBP_CrystalButton _activateactor))
            (EventDispatchers|BindEventtoOnPressedDispatcher _asbp_crystal_button (EventDispatchers|CreateEvent :!event Custom|OnButtonPressed))))))))

(fn ConstructionScript)